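; BP_Maze is the tiltable maze board for a ball maze, rotated by player input.
; The TiltForward and TiltRight axes rotate the SMMaze component in pitch and roll respectively, scaled by RotationSpeed.
; Each step is followed by a clamp that keeps the tilt within five degrees either way.
; Pitch is applied and clamped in world space, while roll is added locally and clamped on relative rotation.
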(event Input|AxisEvents|InputAxisTiltForward
  (params (AxisValue :type Float%20%28single-precision%29))
  (bind _sm_maze (Variables|Default|GetSM_Maze))
  (bind _returnvalue (Transformation|GetWorldRotation _sm_maze))
  (Transformation|AddWorldRotation (Variables|Default|GetSM_Maze) (Math|Rotator|MakeRotator 0.0 (* AxisValue (Variables|Default|GetRotationSpeed)) 0.0) false false)
  (Transformation|SetWorldRotation (Variables|Default|GetSM_Maze) (Math|Rotator|MakeRotator (.roll _returnvalue) (Math|Float|Clamp(Float) (.pitch _returnvalue) -5.0 5.0) (.yaw _returnvalue)) false false))

(event Input|AxisEvents|InputAxisTiltRight
  (params (AxisValue :type Float%20%28single-precision%29))
  (bind _sm_maze (Variables|Default|GetSM_Maze))
  (bind _relativerotation (Variables|/Script/Engine.SceneComponent|GetRelativeRotation _sm_maze))
  (Transformation|AddLocalRotation (Variables|Default|GetSM_Maze) (Math|Rotator|MakeRotator (* AxisValue (Variables|Default|GetRotationSpeed)) 0.0 0.0) false false)
  (Transformation|SetRelativeRotation (Variables|Default|GetSM_Maze) (Math|Rotator|MakeRotator (Math|Float|Clamp(Float) (.roll _relativerotation) -5.0 5.0) (.pitch _relativerotation) (.yaw _relativerotation)) false false))

(fn ConstructionScript)