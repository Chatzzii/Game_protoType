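; BP_Ball is the ball actor for the Ball Maze game.
; On BeginPlay it stores its starting location and binds to the overlap event of its Maze's goal, which teleports it back to the start and zeroes its linear velocity.
; Tick destroys the actor when it falls below a kill height, rather than resetting it.
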(event Custom|OnBallOverlap_Event_0
  (CallFunction|ResetBalltoStart))

(event EventBeginPlay
  (Variables|Default|SetStartingLocation (Transformation|GetActorLocation))
  (EventDispatchers|AssignOnBallOverlap (Default|GetGoal (Variables|Default|GetMaze)) (delegate Custom|OnBallOverlap_Event_0)))

(event EventDestroyed)

(event EventTick
  (params (DeltaSeconds :type Float%20%28single-precision%29))
  (if (< (.z (Transformation|GetActorLocation)) (Variables|Default|GetKillHight))
    (Actor|DestroyActor)))

(fn ConstructionScript)

(fn ResetBalltoStart
  (Transformation|SetActorLocation (Variables|Default|GetStartingLocation) false false)
  (Physics|SetPhysicsLinearVelocity (Variables|Components|GetBALL) "0, 0, 0" false "None"))