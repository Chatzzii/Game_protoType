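; BP_Ball is the ball actor for the Ball Maze game, returning to its start position when it falls out of bounds.
; It records its location on BeginPlay and checks its height against KillHight every Tick.
; Below that height, ResetBallToStart moves the actor back without sweep and zeroes the linear physics velocity of the BALL component, leaving angular velocity untouched.
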(event EventBeginPlay
  (Variables|Default|SetStartingLocation (Transformation|GetActorLocation)))

(event EventTick
  (params (DeltaSeconds :type Float%20%28single-precision%29))
  (if (< (.z (Transformation|GetActorLocation)) (Variables|Default|GetKillHight))
    (CallFunction|ResetBalltoStart)))

(fn ConstructionScript)

(fn ResetBalltoStart
  (Transformation|SetActorLocation (Variables|Default|GetStartingLocation) false false)
  (Physics|SetPhysicsLinearVelocity (Variables|Components|GetBALL) "0, 0, 0" false "None"))